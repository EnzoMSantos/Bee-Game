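; RTS game state that controls game speed, tracks the current day and hour, and adds the GameTime widget to the screen.
; SetGameScaleVelocity sets TimeState, which Tick maps to global time dilation, with X 4 actually applying 10x.
; Tick counters that dilation on its own CustomTimeDilation and reads Hour from the level's SunMoonDaySequenceActor.
; Event_SwitchDay increments the day counter.
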(event Custom|Event_SwitchDay
  (Variables|Default|SetDay (+ (Variables|Default|GetDay) 1)))

(event Custom|GetCurrentTimeOfDay)

(event EventBeginPlay
  (Utilities|FlowControl|Sequence
    (:then_1
      (bind _outactors (Actor|GetAllActorsOfClass "/Script/DaySequence.SunMoonDaySequenceActor"))
      (bind _array_element (Utilities|Array|ForEachLoopwithBreak _outactors :!label _label)
        (:LoopBody
          (Variables|Default|SetDaySequenceActorReference _array_element)
          (goto _label Break))))
    (:then_2
      (bind _returnvalue (UserInterface|CreateWidget "/Game/RTS/UI/GameTime.GameTime_C"))
      (UserInterface|Viewport|AddtoViewport _returnvalue 0))))

(event EventTick
  (params (DeltaSeconds :type Float%20%28single-precision%29))
  (Utilities|FlowControl|Sequence
    (:then_0
      (Variables|Default|SetCustomTimeDilation (/ 1.0 (Class|GameplayStatics|GetGlobalTimeDilation))))
    (:then_2
      (switch Utilities|FlowControl|Switch|SwitchonGameState (Variables|Default|GetTimeState)
        (:NewEnumerator0
          (Utilities|Time|SetGlobalTimeDilation 1.0))
        (:NewEnumerator1
          (Utilities|Time|SetGlobalTimeDilation 0.0))
        (:NewEnumerator2
          (Utilities|Time|SetGlobalTimeDilation 2.0))
        (:NewEnumerator3
          (Utilities|Time|SetGlobalTimeDilation 1e+01))))
    (:then_3
      (Variables|Default|SetHour (Math|Float|Truncate (Class|DaySequenceActor|GetTimeOfDay (Variables|Default|GetDaySequenceActorReference)))))))

(fn ConstructionScript)

(fn SetGameScaleVelocity
  (params (Speed :type GameState%20Enum :default "NewEnumerator0"))
  (Variables|Default|SetTimeState Speed))